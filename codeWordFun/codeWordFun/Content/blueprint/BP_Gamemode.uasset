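; BP_Gamemode is a game mode that drives the monster audio, switching from ambiance to the SC_chris sound based on the player's cassette timer.
; BeginPlay spawns both 2D sounds without auto-destroy.
; Each Tick, a negative TimerByCasette on BP_Character activates SC_chris and deactivates ambiance; otherwise SC_chris fades out and deactivates after a short Delay.
; Ambiance is never reactivated once switched off.
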(event `self.ReceiveBeginPlay`
  ;[1 1 1] Audio for monster
  (bind _returnvalue (`GameplayStatics.SpawnSound2D` "/Game/SFX/SFXQues/SC_Ambiance.SC_Ambiance" 3.0 1.0 0.0 null false false))
  (`ActorComponent.SetActive` _returnvalue true false)
  (bind _returnvalue_2 (`GameplayStatics.SpawnSound2D` "/Game/SFX/SFXQues/SC_chris.SC_chris" 1.0 1.0 0.0 null false false)))

(event `self.ReceiveTick`
  (params (DeltaSeconds :type "Float (single-precision)"))
  ;[1 1 1] Audio for monster
  (bind _asbp_character (cast `/Game/blueprint/BP_Character` (`GameplayStatics.GetPlayerCharacter` 0)))
  (if (< (`/Game/blueprint/BP_Character.TimerByCasette` _asbp_character) 0.0)
    (`ActorComponent.SetActive` (stale `self.ReceiveBeginPlay` _returnvalue_2) true false)
    (`ActorComponent.SetActive` (stale `self.ReceiveBeginPlay` _returnvalue) false false)
    (else
      (`AudioComponent.FadeOut` (stale `self.ReceiveBeginPlay` _returnvalue_2) 0.4 0.0 "Logarithmic")
      (`KismetSystemLibrary.Delay` 0.4)
      (`ActorComponent.SetActive` (stale `self.ReceiveBeginPlay` _returnvalue_2) false false))))

(fn `UserConstructionScript`)