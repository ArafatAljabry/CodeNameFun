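; BP_monster is a monster actor that glides toward the player and catches them.
; On BeginPlay it caches the player BP_Character, snapshots the world location of its CloseTarget component once, and starts ambiance and SC_chris 2D sounds.
; Tick moves it at constant speed to that fixed point without sweeping, then calls MonsterCaughtPlayer on the player every frame it is within a small distance of the point.
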(event `self.ReceiveBeginPlay`
  (bind _asbp_character (cast `/Game/blueprint/BP_Character` (`GameplayStatics.GetPlayerPawn` 0)))
  (bind _output_get (set `self.Player` _asbp_character))
  (set `self.Close point` (`SceneComponent.K2_GetComponentLocation` (`/Game/blueprint/BP_Character.close target` _output_get)))
  (bind _returnvalue (`GameplayStatics.SpawnSound2D` "/Game/SFX/SFXQues/SC_Ambiance.SC_Ambiance" 3.0 1.0 0.0 null false false))
  (`ActorComponent.SetActive` _returnvalue true false)
  (`GameplayStatics.SpawnSound2D` "/Game/SFX/SFXQues/SC_chris.SC_chris" 1.0 1.0 0.0 null false false))

(event `self.ReceiveTick`
  (params (DeltaSeconds :type "Float (single-precision)"))
  (`/Engine/EditorBlueprintResources/StandardMacros.IsValid` (`self.Player`)
    (:`Is Valid`
      (`self.K2_SetActorLocation` (`KismetMathLibrary.VInterpTo_Constant` (`SceneComponent.K2_GetComponentLocation` (`self.DefaultSceneRoot`)) (`self.Close point`) DeltaSeconds 300.0))
      (if (< (`KismetMathLibrary.Vector_Distance` (`SceneComponent.K2_GetComponentLocation` (`self.DefaultSceneRoot`)) (`self.Close point`)) 10.0)
        (bind _asbp_character (cast `/Game/blueprint/BP_Character` (`GameplayStatics.GetPlayerPawn` 0)))
        (`/Game/blueprint/BP_Character.MonsterCaughtPlayer` _asbp_character)))))

(fn `UserConstructionScript`)