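; BP_Casette is an interactable cassette actor that is destroyed when the player interacts with it.
; It creates a WB_Interact widget on BeginPlay and shows or removes it as the player character enters or leaves its Sphere overlap.
; The Interact event plays a 2D camera shutter sound and destroys the actor, with no overlap check of its own.
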(event `self.ReceiveBeginPlay`
  ;[1 1 1] UI
  (bind _returnvalue (`|CreateWidget` "/Game/blueprint/WB_Interact.WB_Interact_C"))
  (set `self.InteractWidget` _returnvalue))

(event `self.Sphere.OnComponentBeginOverlap`
  (params (OverlappedComponent :type "PrimitiveComponent Object Reference") (OtherActor :type "Actor Object Reference") (OtherComp :type "PrimitiveComponent Object Reference") (OtherBodyIndex :type Integer) (bFromSweep :type Boolean) (SweepResult :type "HitResult Structure (by ref)"))
  ;[1 1 1] Interaction pop-up
  (if (== OtherActor (`GameplayStatics.GetPlayerCharacter` 0))
    (`UserWidget.AddToViewport` (`self.InteractWidget`) 0)))

(event `self.Sphere.OnComponentEndOverlap`
  (params (OverlappedComponent :type "PrimitiveComponent Object Reference") (OtherActor :type "Actor Object Reference") (OtherComp :type "PrimitiveComponent Object Reference") (OtherBodyIndex :type Integer))
  ;[1 1 1] Interaction pop-up
  (if (== (`GameplayStatics.GetPlayerCharacter` 0) OtherActor)
    (`Widget.RemoveFromParent` (`self.InteractWidget`))))

(event `/Game/blueprint/I_Interactable.Interact`
  ;[1 1 1] Destroy cassett
  (`GameplayStatics.PlaySound2D` "/Engine/VREditor/Sounds/UI/Camera_Shutter.Camera_Shutter" 1.0 1.0 0.0 null null)
  (`self.K2_DestroyActor`))

(fn `UserConstructionScript`)